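; Timer Blueprint that runs a level countdown and opens the EndScreen level when time runs out.
; On BeginPlay it starts a looping one-second timer that calls Decrement by function name.
; Decrement lowers TimerValue by one, clamps it at zero, prints the remaining value to screen, and loads EndScreen once it reaches zero.
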(event EventBeginPlay
  (Utilities|Time|SetTimerbyFunctionName 0 "Decrement" 1.0 true))

(fn ConstructionScript)

(fn Decrement
  (bind _output_get (Variables|Default|SetTimerValue (Math|Integer|Clamp(Integer) (- (Variables|Default|GetTimerValue) 1) 0 (Variables|Default|GetTimerValue))))
  (Development|PrintString (Utilities|String|ToString(Integer) _output_get))
  (if (<= (Variables|Default|GetTimerValue) 0)
    (Game|OpenLevel(byName) "EndScreen")))