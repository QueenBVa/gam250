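; Unit manager for a turn-based game that populates generated rooms with both teams, the possessed player pawn and an end pickup.
; BuildUnits filters rooms by area, picks a random player room, then spawns enemies in groups elsewhere.
; SpawnLocations retries random grid cells, and spawned units mark theirs blocked in PathFinder.
; Enemy stats come from random points and derived formulas stored in StatBlock, though spawned units receive DefaultStatBlock.
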(event Custom|GenerateBasicEnemyTeam
  (bind _teamsize (Variables|Default|GetTeamSize))
  (bind _output (Utilities|Array|Get(acopy) _teamsize))
  ;[1 1 1] Get the team sizes, and figure out where the enemy stat blocks should begin, the loop through them to create their stat blocks
  (Variables|UnitStats|SetTeam 1)
  (for _index (range _output (+ (Utilities|Array|Get(acopy) (Variables|Default|GetTeamSize) 1) (- _output 1)))
    (CallFunction|GetUnitStatBlock _index)
    ;[1 1 1] Creates the Unit's basic stats
    (for _index_2 (range 1 (+ (Variables|Default|GetDefaultPoints) 0))
      (switch int (Math|Random|RandomIntegerinRange 0 3)
        (:Default
          (Variables|UnitStats|SetStrength (+ (Variables|UnitStats|GetStrength) 1) :!label _label))
        (:0
          (goto _label))
        (:1
          (Variables|UnitStats|SetIntelligence (+ (Variables|UnitStats|GetIntelligence) 1)))
        (:2
          (Variables|UnitStats|SetDexterity (+ (Variables|UnitStats|GetDexterity) 1)))
        (:3
          (Variables|UnitStats|SetConstitution (+ (Variables|UnitStats|GetConstitution) 1)))))
    ;[1 1 1] Calculate the Derived values then set the enemy unit's healt to max (as they are just now generated and not loaded
    (CallFunction|CalculateDerivedValues)
    (CallFunction|SetStartingHealthandPower)
    ;[1 1 1] Store all these values into the stat block
    (CallFunction|SetUnitStatBlock _index)))

(event Custom|InitUnitArrays
  (bind _statblock (Variables|UnitStats|GetStatBlock))
  (bind _mapsize (Variables|Default|GetMapSize))
  (bind _statblock_2 (Variables|UnitStats|GetStatBlock))
  (bind _x (Math|Vector|BreakVector _mapsize))
  (bind _returnvalue (Math|Float|Floor _x))
  ;[1 1 1] Called at the beginning of  BuildUnits, this just resets the Stat Block array and gets it ready to accept new values
  (Utilities|Array|SetArrayElem (Variables|Default|GetTeamSize) 1 (Math|Integer|SelectInt _returnvalue 32 (<= _returnvalue 32)))
  ;;[1 1 1] Creates and Resets the Stat Block Array, based on the total number of units
  (Utilities|Array|Clear _statblock_2)
  (Utilities|Array|Resize _statblock_2 (+ (Utilities|Array|Get(acopy) (Variables|Default|GetTeamSize) 1) (Utilities|Array|Get(acopy) (Variables|Default|GetTeamSize))))
  (for (_ _array_index) _statblock
    (Utilities|Array|SetArrayElem _statblock _array_index (Variables|Default|GetDefaultStatBlock))))

(event Custom|BuildUnits
  (params (RoomsIn :type Array%20of%20AABB%20Object%20References))
  (bind _returnvalue (Game|GetPlayerController 0))
  (bind _teamsize (Variables|Default|GetTeamSize))
  (bind _playerstartrooms (Variables|Default|GetPlayerStartRooms))
  (bind _bigenoughrooms (Variables|Default|GetBigEnoughRooms))
  (bind _bigenoughrooms_2 (Variables|Default|GetBigEnoughRooms))
  (bind _output (Utilities|Array|Get(acopy) _teamsize))
  (CallFunction|InitUnitArrays)
  (Variables|Default|SetRooms RoomsIn)
  ;[1 1 1] Cycle through the rooms, discard any room less than size of the number of units on the team being spawned
  (for _array_element (Variables|Default|GetRooms)
    (bind _area (CallFunction|RoomArea _array_element))
    (if (> _area (* (Utilities|Array|Get(acopy) (Variables|Default|GetTeamSize) 1) 1))
      (Utilities|Array|Add (Variables|Default|GetBigEnoughRooms) _array_element)))
  (CallFunction|PlaceEndPoint)
  ;[1 1 1] Now, of those rooms, filter then down to the rooms the Player's team can spawn into
  (for _array_element_2 (Variables|Default|GetBigEnoughRooms)
    (bind _area_2 (CallFunction|RoomArea _array_element_2))
    (if (> _area_2 (* (Utilities|Array|Get(acopy) (Variables|Default|GetTeamSize)) 2))
      (Utilities|Array|Add (Variables|Default|GetPlayerStartRooms) _array_element_2)))
  ;[1 1 1] Randomly choose the Player's Team Starting room.
  (Variables|Default|SetPlayerRoomStartIndex (Math|Random|RandomIntegerinRange 0 (- (Utilities|Array|Length _playerstartrooms) 1)))
  (Variables|Default|SetPlayerStartRoom (Utilities|Array|Get(acopy) _playerstartrooms (Variables|Default|GetPlayerRoomStartIndex)))
  (Utilities|Array|RemoveItem (Variables|Default|GetBigEnoughRooms) (Variables|Default|GetPlayerStartRoom))
  ;[1 1 1] Spawn the Player's Team and the Player's Pawn (and possess it)
  (bind _outputlocations (CallFunction|SpawnLocations (Variables|Default|GetPlayerStartRoom) (Utilities|Array|Get(acopy) (Variables|Default|GetTeamSize))))
  (for _array_element_3 _outputlocations
    (bind _returnvalue_2 (AI|SpawnAIFromClass "/Game/Units/Unit.Unit_C" 0 _array_element_3 "0, 0, 0" true))
    (bind _asunit (Utilities|Casting|CastToUnit _returnvalue_2))
    (Variables|/Game/Units/Unit.Unit_C|SetStatBlock _asunit (Variables|Default|GetDefaultStatBlock))
    (Default|SetStatVars _asunit)
    (Utilities|Array|Add (Variables|Default|GetAllUnits) _asunit)
    (Variables|/Game/Units/Unit.Unit_C|SetTeam _asunit 0)
    (Default|GridChangeVector (Variables|Default|GetPathFinder) (Transformation|GetActorLocation _returnvalue_2) -1))
  (bind _returnvalue_3 (Game|SpawnActorfromClass "/Game/Blueprints/Game/TBS_PlayerPawn.TBS_PlayerPawn_C" (Math|Transform|MakeTransform (Transformation|GetActorLocation (Variables|Default|GetPlayerStartRoom))) "AlwaysSpawn" 0 0))
  (Pawn|Possess _returnvalue _returnvalue_3)
  (bind _asmain_player_controller (Utilities|Casting|CastToMainPlayerController _returnvalue))
  (Variables|/Game/Blueprints/Game/MainPlayerController.MainPlayerController_C|SetPathFinder _asmain_player_controller (Variables|Default|GetPathFinder))
  ;[1 1 1] Now gerenate the Enemy Team
  (Variables|Default|SetTeamIndex 1)
  (CallFunction|GenerateBasicEnemyTeam)
  ;[1 1 1] Randomly choose some rooms, and spawn the enemy units in groups (like 4-5)
  (for _index (range _output (/ (+ (Utilities|Array|Get(acopy) (Variables|Default|GetTeamSize) 1) (- _output 1)) (Variables|Default|GetUnitsPerRoom)))
    (Variables|Default|SetCounter (Math|Random|RandomIntegerinRange 0 (- (Utilities|Array|Length _bigenoughrooms_2) 1)))
    (if (== (Utilities|Array|Get(acopy) _bigenoughrooms_2 (Variables|Default|GetCounter)) (Variables|Default|GetPlayerStartRoom))
      (Utilities|Array|RemoveIndex _bigenoughrooms (Variables|Default|GetCounter))
      (if (== (Variables|Default|GetCounter) 0)
        _
        (elif (== (Utilities|Array|LastIndex _bigenoughrooms) (Variables|Default|GetCounter))
          (Variables|Default|SetCounter (- (Variables|Default|GetCounter) 1))))
      (bind _outputlocations_2 (CallFunction|SpawnLocations (Utilities|Array|Get(acopy) _bigenoughrooms_2 (Variables|Default|GetCounter)) (Variables|Default|GetUnitsPerRoom) :!label _label))
      (Utilities|Array|RemoveIndex (Variables|Default|GetBigEnoughRooms) (Variables|Default|GetCounter))
      (for (_array_element_4 _array_index) _outputlocations_2
        (bind _returnvalue_4 (AI|SpawnAIFromClass "/Game/Units/Unit.Unit_C" 0 _array_element_4 "0, 0, 0" true))
        (bind _asunit_2 (Utilities|Casting|CastToUnit _returnvalue_4))
        (Variables|/Game/Units/Unit.Unit_C|SetStatBlock _asunit_2 (Variables|Default|GetDefaultStatBlock))
        (Default|SetStatVars _asunit_2)
        (Rendering|SetActorHiddenInGame _asunit_2 false) ; Currently Disabled: Hide the unit in prep for LOS
        (Utilities|Array|Add (Variables|Default|GetAllUnits) _asunit_2)
        (Variables|/Game/Units/Unit.Unit_C|SetTeam _asunit_2 1)
        (Default|GridChangeVector (Variables|Default|GetPathFinder) (Transformation|GetActorLocation _asunit_2) -1))
      (else
        (Utilities|IsValid (Utilities|Array|Get(acopy) _bigenoughrooms_2 (Variables|Default|GetCounter))
          (:Is%20Valid
            (goto _label))
          (:Is%20Not%20Valid
            (Development|PrintString "BigEnoughRoomNotValid")))))))

(event EventBeginPlay)

(fn ConstructionScript
  (bind _unitstatblock (Utilities|Struct|MakeUnitStatBlock 5 5))
  (Variables|Default|SetTempStatBlock _unitstatblock)
  (Variables|Default|SetDefaultStatBlock _unitstatblock))

(fn SpawnLocations
  (params (InputRoom :type AABB%20Object%20Reference) (NumberOfSpawns :type Integer))
  (bind _returnvalue (Transformation|GetActorLocation InputRoom))
  (bind _aabb (Variables|/Game/Blueprints/QuadTree/AABB.AABB_C|GetAABB InputRoom))
  (bind _boxextent (Variables|/Script/Engine.BoxComponent|GetBoxExtent _aabb))
  (bind _returnvalue_2 (- _returnvalue _boxextent))
  (bind _returnvalue_3 (+ _returnvalue _boxextent))
  (bind _returnvalue_4 (/ _returnvalue_2 1e+02))
  (bind _returnvalue_5 (/ _returnvalue_3 1e+02))
  (bind (_x _y) (Math|Vector|BreakVector _returnvalue_4))
  (bind (_x_2 _y_2) (Math|Vector|BreakVector _returnvalue_5))
  (bind _returnvalue_6 (Math|Float|Floor _x))
  (bind _returnvalue_7 (Math|Float|Floor _y))
  (bind _returnvalue_8 (Math|Float|Floor _y_2))
  (bind _returnvalue_9 (Math|Float|Floor _x_2))
  (bind _returnvalue_10 (- _returnvalue_8 1))
  (bind _returnvalue_11 (- _returnvalue_9 1))
  (bind _returnvalue_12 (Math|Random|RandomIntegerinRange _returnvalue_7 _returnvalue_10))
  (bind _returnvalue_13 (Math|Random|RandomIntegerinRange _returnvalue_6 _returnvalue_11))
  ;[1 1 1] Randomly select a grid space in the room to spawn a unit, store it, then loop back, if a space is already chosen, don't allow another to choose it.
  (Utilities|Array|Clear (Variables|Default|GetReturnLocations))
  (Variables|Default|SetNumberOfUnits NumberOfSpawns)
  (for _index (range 1 (Variables|Default|GetNumberOfUnits))
    (Utilities|FlowControl|ForLoopwithBreak 0 15 :!label _label
      (:LoopBody
        (Variables|Default|SetTemp (Math|Vector|MakeVector (Math|Conversions|ToFloat(Integer) (+ (* _returnvalue_13 100) 50)) (Math|Conversions|ToFloat(Integer) (+ (* _returnvalue_12 100) 50)) 0.0))
        (if (not (Utilities|Array|ContainsItem (Variables|Default|GetReturnLocations) (Variables|Default|GetTemp)))
          (if (not (== (Utilities|Array|Get(acopy) (Variables|/Game/Blueprints/A-Star/PathFinder.PathFinder_C|GetmGrid (Variables|Default|GetPathFinder)) (+ (* (Math|Float|Floor (.Y (Math|Vector|BreakVector (Variables|Default|GetMapSize)))) _returnvalue_12) _returnvalue_13)) -1))
            (Utilities|Array|Add (Variables|Default|GetReturnLocations) (Variables|Default|GetTemp))
            (goto _label Break))))))
  (return (Variables|Default|GetReturnLocations)))

(fn RoomArea
  (params (InputAABB :type AABB%20Object%20Reference))
  (bind _aabb (Variables|/Game/Blueprints/QuadTree/AABB.AABB_C|GetAABB InputAABB))
  (bind _boxextent (Variables|/Script/Engine.BoxComponent|GetBoxExtent _aabb))
  (bind _returnvalue (* _boxextent 2.0))
  (bind _returnvalue_2 (/ _returnvalue 1e+02))
  (bind (_x _y) (Math|Vector|BreakVector _returnvalue_2))
  (return (Math|Float|Floor (* _x _y))))

(fn DestroyUnit
  (params (UnitToDestroy :type Unit%20Object%20Reference))
  (bind _allunits (Variables|Default|GetAllUnits))
  (Utilities|Array|RemoveIndex _allunits (Utilities|Array|FindItem _allunits UnitToDestroy))
  (Actor|DestroyActor UnitToDestroy))

(fn SetUnitStatBlock
  (params (Index :type Integer))
  ;[1 1 1] Sets the Unit's Stat block within the Stat Block Array
  (Utilities|Struct|SetmembersinUnitStatBlock (Variables|Default|GetTempStatBlock) (Variables|UnitStats|GetStrength) (Variables|UnitStats|GetIntelligence) (Variables|UnitStats|GetDexterity) (Variables|UnitStats|GetConstitution) (Variables|UnitStats|GetHealth) (Variables|UnitStats|GetCurrentHealth) (Variables|UnitStats|GetPower) (Variables|UnitStats|GetCurrentPower) (Variables|UnitStats|GetSpeed) (Variables|UnitStats|GetCurrentSpeed) (Variables|UnitStats|GetMaxSightRange) (Variables|UnitStats|GetCurrentSightRange) (Variables|UnitStats|GetCanAct) (Variables|UnitStats|GetHasActed) (Variables|UnitStats|GetIsDisabled) (Variables|UnitStats|GetCanMove) (Variables|UnitStats|GetHasMoved) (Variables|UnitStats|GetIsRooted) (Variables|UnitStats|GetTeam) (Variables|UnitStats|GetMovementRange) (Variables|UnitStats|GetNumberOfMoves) (Variables|UnitStats|GetCurrentMovementRange) (Variables|UnitStats|GetMeleeBaseAttack) (Variables|UnitStats|GetRangedBaseAttack) (Variables|UnitStats|GetMagicBaseAttack) (Variables|UnitStats|GetMeleeBaseDamage) (Variables|UnitStats|GetRangedBaseDamage) (Variables|UnitStats|GetMagicBaseDamage) (Variables|UnitStats|GetBaseDamageAbsorb) (Variables|UnitStats|GetBaseDamageAvoidance) (Variables|UnitStats|GetBaseMagicResist) (Variables|UnitStats|GetBaseMagicPenetration) (Variables|UnitStats|GetCurrentDamageAbsorb) (Variables|UnitStats|GetCurrentDamageAvoidance) (Variables|UnitStats|GetCurrentMagicResist) (Variables|UnitStats|GetCurrentMagicPenetration))
  (Utilities|Array|SetArrayElem (Variables|UnitStats|GetStatBlock) Index (Variables|Default|GetTempStatBlock)))

(fn CalculateDerivedValues
  (bind _strength (Variables|UnitStats|GetStrength))
  (bind _dexterity (Variables|UnitStats|GetDexterity))
  (bind _intelligence (Variables|UnitStats|GetIntelligence))
  (bind _dexterity_2 (Variables|UnitStats|GetDexterity))
  (bind _strength_2 (Variables|UnitStats|GetStrength))
  (bind _returnvalue (>= _strength _intelligence))
  (bind _returnvalue_2 (+ _strength_2 _dexterity_2))
  (bind _returnvalue_3 (Math|Integer|SelectInt _strength _intelligence _returnvalue))
  ;[1 1 1] Calculates all the dervived stats from just the 4 base stats
  (if (and (<= _returnvalue_2 17) (>= _returnvalue_2 10))
    (Variables|UnitStats|SetSpeed 6e+02)
    (elif (> _returnvalue_2 17)
      (Variables|UnitStats|SetSpeed 7.5e+02)
      (else
        (Variables|UnitStats|SetSpeed 4.5e+02))))
  (Variables|UnitStats|SetHealth (* (+ (* (Variables|UnitStats|GetConstitution) 1.75) (* (Variables|UnitStats|GetStrength) 0.65)) 5.0))
  (Variables|UnitStats|SetPower (* (Math|Integer|SelectInt _returnvalue_3 _dexterity (>= _returnvalue_3 _dexterity)) 5.0))
  (Variables|UnitStats|SetNumberOfMoves (/ (Variables|UnitStats|GetConstitution) 4))
  (Variables|UnitStats|SetMovementRange (/ (Variables|UnitStats|GetDexterity) 4))
  (Variables|UnitStats|SetCurrentMovementRange (* (Variables|UnitStats|GetMovementRange) (Variables|UnitStats|GetNumberOfMoves)))
  (Variables|UnitStats|SetCurrentMagicResist (+ (* (Variables|UnitStats|GetIntelligence) 1.25) (Variables|UnitStats|GetBaseMagicResist)))
  (Variables|UnitStats|SetCurrentDamageAvoidance (+ (* (Variables|UnitStats|GetDexterity) 1.25) (Variables|UnitStats|GetBaseDamageAvoidance)))
  (Variables|UnitStats|SetCurrentMagicPenetration (+ (* (Variables|UnitStats|GetIntelligence) 1.0) (Variables|UnitStats|GetBaseMagicPenetration)))
  (Variables|UnitStats|SetCurrentDamageAbsorb (+ (* (Variables|UnitStats|GetConstitution) 0.65) (* (Variables|UnitStats|GetStrength) 0.65) (Variables|UnitStats|GetBaseDamageAbsorb)))
  (Variables|UnitStats|SetMagicBaseAttack (Math|Float|Floor (* (Variables|UnitStats|GetIntelligence) 2.5)))
  (Variables|UnitStats|SetRangedBaseAttack (Math|Float|Floor (* (Variables|UnitStats|GetDexterity) 2.5)))
  (Variables|UnitStats|SetMeleeBaseAttack (Math|Float|Floor (* (Variables|UnitStats|GetStrength) 2.5)))
  (Variables|UnitStats|SetMagicBaseDamage (* (+ (Variables|UnitStats|GetIntelligence) 25) 1.65))
  (Variables|UnitStats|SetRangedBaseDamage (* (+ (Variables|UnitStats|GetDexterity) 25) 1.65))
  (Variables|UnitStats|SetMeleeBaseDamage (* (+ (Variables|UnitStats|GetStrength) 25) 1.65)))

(fn GetUnitStatBlock
  (params (Index :type Integer))
  (bind _statblock (Variables|UnitStats|GetStatBlock))
  (bind _output (Utilities|Array|Get(acopy) _statblock Index))
  (bind (_strength _intelligence _dexterity _constitution _maxhealth _currenthealth _maxpower _currentpower _maxspeed _currentspeed _maxsightrange _currentsightrange _bcanact _bhasacted _bisdisabled _bcanmove _bhasmoved _bisrooted _team _rangepermove _numberofmoves _currenttotalmovementrnage _meleebaseattack _rangedbaseattack _magicbaseattack _meleebasedamage _rangedbasedamage _magicbasedamage _basedamageabsorb _basedamageavoidance _basemagicresist _basemagicpenetration _currentdamageabsorb _currentdamageavoidance _currentmagicresist _currentmagicpenetration) (Utilities|Struct|BreakUnitStatBlock _output))
  ;[1 1 1] Very simply breaks the Unit's stat block and sets a bunch of variables to be more easily worked with
  (Variables|UnitStats|SetStrength _strength)
  (Variables|UnitStats|SetIntelligence _intelligence)
  (Variables|UnitStats|SetDexterity _dexterity)
  (Variables|UnitStats|SetConstitution _constitution)
  (Variables|UnitStats|SetHealth _maxhealth)
  (Variables|UnitStats|SetCurrentHealth _currenthealth)
  (Variables|UnitStats|SetPower _maxpower)
  (Variables|UnitStats|SetCurrentPower _currentpower)
  (Variables|UnitStats|SetSpeed _maxspeed)
  (Variables|UnitStats|SetCurrentSpeed _currentspeed)
  (Variables|UnitStats|SetMaxSightRange _maxsightrange)
  (Variables|UnitStats|SetCurrentSightRange _currentsightrange)
  (Variables|UnitStats|SetCanAct _bcanact)
  (Variables|UnitStats|SetHasActed _bhasacted)
  (Variables|UnitStats|SetIsDisabled _bisdisabled)
  (Variables|UnitStats|SetCanMove _bcanmove)
  (Variables|UnitStats|SetHasMoved _bhasmoved)
  (Variables|UnitStats|SetIsRooted _bisrooted)
  (Variables|UnitStats|SetTeam _team)
  (Variables|UnitStats|SetMovementRange _rangepermove)
  (Variables|UnitStats|SetNumberOfMoves _numberofmoves)
  (Variables|UnitStats|SetCurrentMovementRange _currenttotalmovementrnage)
  (Variables|UnitStats|SetMeleeBaseAttack _meleebaseattack)
  (Variables|UnitStats|SetRangedBaseAttack _rangedbaseattack)
  (Variables|UnitStats|SetMagicBaseAttack _magicbaseattack)
  (Variables|UnitStats|SetMeleeBaseDamage _meleebasedamage)
  (Variables|UnitStats|SetRangedBaseDamage _rangedbasedamage)
  (Variables|UnitStats|SetMagicBaseDamage _magicbasedamage)
  (Variables|UnitStats|SetBaseDamageAbsorb _basedamageabsorb)
  (Variables|UnitStats|SetBaseDamageAvoidance _basedamageavoidance)
  (Variables|UnitStats|SetBaseMagicResist _basemagicresist)
  (Variables|UnitStats|SetBaseMagicPenetration _basemagicpenetration)
  (Variables|UnitStats|SetCurrentDamageAbsorb _currentdamageabsorb)
  (Variables|UnitStats|SetCurrentDamageAvoidance _currentdamageavoidance)
  (Variables|UnitStats|SetCurrentMagicResist _currentmagicresist)
  (Variables|UnitStats|SetCurrentMagicPenetration _currentmagicpenetration))

(fn SetStartingHealthandPower
  ;[1 1 1] For fully healed units, or new ones
  (Variables|UnitStats|SetCurrentHealth (Variables|UnitStats|GetHealth))
  (Variables|UnitStats|SetCurrentPower (Variables|UnitStats|GetPower)))

(fn PlaceEndPoint
  (bind _rooms (Variables|Default|GetRooms))
  (bind _outputlocations (CallFunction|SpawnLocations (Utilities|Array|Get(acopy) _rooms (Math|Random|RandomIntegerinRange 0 (Utilities|Array|Length _rooms))) 1))
  (Game|SpawnActorfromClass "/Game/Blueprints/EndPickup.EndPickup_C" (Math|Transform|MakeTransform (Utilities|Array|Get(acopy) _outputlocations)) "Undefined" 0 0))